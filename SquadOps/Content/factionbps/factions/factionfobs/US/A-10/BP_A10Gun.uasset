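; A-10 gun run strike actor that strafes a target location with radio chatter, flyover and cannon effects.
; The server positions the gun high, offset along the attack direction, while clients spawn a BP_A10Flyover.
; After timed delays, a rotating sweep of randomized line traces precomputes impact points, then replayed for explosion effects and radial damage.
; The cannon sound plays on clients after the impacts, mimicking delayed audio, before the server destroys the actor.
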(event Custom|Explode
  ;[1 1 1] Splash effect and sounds on every client, damage effect on server
  (bind _index (Utilities|ForLoopwithDelay 1 (- (Utilities|Array|Length (Variables|Default|GetHitArray)) 1) 0.0)
    (:Loop%20Body
      (Audio|PlaySoundatLocation "/SquadOps/factionbps/factions/factionfobs/US/A-10/A10Hit.A10Hit" (Utilities|Array|Get(acopy) (Variables|Default|GetHitArray) _index) "0, 0, 0" 1.0)
      (Effects|SpawnEmitteratLocation "/SquadOps/factionbps/factions/factionfobs/US/A-10/A10_GAU_Impact.A10_GAU_Impact" (Utilities|Array|Get(acopy) (Variables|Default|GetHitArray) _index)))))

(event Custom|BRRRRT
  ;[1 1 1] Plays sound for all clients, waits, then  destroys the gun
  (Networking|SwitchHasAuthority
    (:Authority
      (Utilities|FlowControl|Delay 2.0)
      (Actor|DestroyActor))
    (:Remote
      ;[1 1 1] BRRRRRRRRRRRRRRRRRRRRRRRRRRRRRRRRRT
      (Audio|SpawnSoundatLocation "/SquadOps/factionbps/factions/factionfobs/US/A-10/Sounds/Fire/Far/gau9_fire_Cue.gau9_fire_Cue" (Transformation|GetActorLocation) "0, 0, 0" 2.0))))

(event Custom|Airplane%20Sound
  (bind _returnvalue (Transformation|GetActorLocation))
  ;[1 1 1] Airplane sound effects
  (Networking|SwitchHasAuthority
    (:Remote
      (Audio|PlaySoundatLocation "/SquadOps/factionbps/factions/factionfobs/US/A-10/Sounds/Flyby/A10_flyover_Cue.A10_flyover_Cue" _returnvalue "0, 0, 0" 0.4)
      (Utilities|FlowControl|Delay 2.0)
      (Audio|PlaySoundatLocation "/SquadOps/factionbps/factions/factionfobs/US/A-10/Sounds/Flyby/A10_flyover_Cue.A10_flyover_Cue" _returnvalue "0, 0, 0" 0.4))))

(event Custom|Play%20Beginning%20Sounds.
  (params (Player :type Player%20Controller%20Object%20Reference))
  (bind _returnvalue (Transformation|GetActorLocation Player))
  ;[1 1 1] Radio Chatter
  (Audio|PlaySoundatLocation "/Game/Audio/Deployables/FOB/Radios/US/military_chatter_14_Cue.military_chatter_14_Cue" _returnvalue)
  (Utilities|FlowControl|Delay 1e+01)
  (Audio|PlaySoundatLocation "/Game/Audio/Deployables/FOB/Radios/US/military_chatter_16_Cue.military_chatter_16_Cue" _returnvalue))

(event Custom|Move%20Gun/Spawn%20Plane
  (params (Direction :type Rotator) (Hitloc :type Vector))
  ;[1 1 1] Calculate Positions
  (Networking|SwitchHasAuthority
    (:Authority
      (Transformation|SetActorTransform (Utilities|MakeTransformfromRotandHitPos Hitloc Direction 2e+04 -2e+04) false true))
    (:Remote
      (bind _returnvalue (Game|SpawnActorfromClass "/SquadOps/factionbps/factions/factionfobs/US/A-10/BP_A10Flyover.BP_A10Flyover_C" (Utilities|MakeTransformfromRotandHitPos Hitloc Direction 3.5e+05 -5e+05) "Undefined" 0 0))
      (Default|StartRun _returnvalue false))))

(event Custom|Begin%20Gunrun
  (params (Direction :type Rotator) (Hitloc :type Vector) (PlayerReference :type Player%20Controller%20Object%20Reference))
  (bind _returnvalue (Transformation|GetActorLocation))
  ;[1 1 1] Trace all impacts before hand
  (CallFunction|MoveGun/SpawnPlane Direction Hitloc)
  (CallFunction|PlayBeginningSounds. PlayerReference)
  (Utilities|FlowControl|Delay 8.0)
  (CallFunction|AirplaneSound)
  (Utilities|FlowControl|Delay 7.0)
  (Transformation|AddActorLocalRotation "-1.500000, 0, 0" false false)
  (for _index (range 1 60)
    (bind _outhit (Collision|LineTraceByChannel _returnvalue (+ _returnvalue (* (Utilities|Innacuracy 1.5) 999999999.0)) "TraceTypeQuery1" false 0 "None"))
    (Utilities|Array|Add (Variables|Default|GetHitArray) (.Location (Collision|BreakHitResult _outhit)))
    (Transformation|AddActorLocalRotation "0.050000, 0, 0" false false))
  ;[1 1 1] Splash effect and sounds on every client, damage effect on server
  (CallFunction|Explode)
  (bind _index_2 (Utilities|ForLoopwithDelay 1 (- (Utilities|Array|Length (Variables|Default|GetHitArray)) 1) 0.0)
    (:Loop%20Body
      (Class|SQBlueprintLibrary|ApplyRadialDamagewithFalloff 1e+02 0.0 (Utilities|Array|Get(acopy) (Variables|Default|GetHitArray) _index_2) 4e+02 5e+02 1e+03 1.0 "/Game/Gameplay/DamageTypes/BP_IED.BP_IED_C" 0 0 0 true "ECC_GameTraceChannel8"))
    (:Completed
      ;[1 1 1] Plays sound for all clients, waits, then  destroys the gun
      (Utilities|FlowControl|Delay 2.0)
      (CallFunction|BRRRRT))))

(fn ConstructionScript)