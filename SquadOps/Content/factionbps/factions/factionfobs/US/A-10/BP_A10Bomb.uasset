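; A-10 bombing run actor that delivers a delayed airstrike on a called location, with radio chatter and jet flyby sounds.
; Authority moves it high above the target, facing it, while remotes spawn a BP_A10Flyover plane.
; After the delays it pre-traces five randomly spread impacts, then staggers explosion effects, camera shake and radial damage over three.
; The authority destroys the actor afterwards.
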(event Custom|Explode
  ;[1 1 1] Splash effect and sounds on every client, damage effect on server
  (bind _index (Utilities|ForLoopwithDelay 2 4 0.2)
    (:Loop%20Body
      (Audio|PlaySoundatLocation "/Game/Weapons/IED/Sounds/Explosion/SC_IED_exp.SC_IED_exp" (Utilities|Array|Get(acopy) (Variables|Default|GetHit) _index) "0, 0, 0" 3.0)
      (Audio|PlaySoundatLocation "/Game/Audio/Impacts/Explosions/Debris/IED/Dirt/Exp_debris_dirt_IED_Cue.Exp_debris_dirt_IED_Cue" (Utilities|Array|Get(acopy) (Variables|Default|GetHit) _index) "0, 0, 0" 3.0)
      (Effects|SpawnEmitteratLocation "/Game/Particles/Explosions/Mine/ATMine_Explosion_Sand.ATMine_Explosion_Sand" (Utilities|Array|Get(acopy) (Variables|Default|GetHit) _index))
      (Camera|PlayWorldCameraShake "/Game/Blueprints/Effects/ShockwaveCameraShake_Short.ShockwaveCameraShake_Short_C" (Utilities|Array|Get(acopy) (Variables|Default|GetHit) _index) 3e+03 2.5e+04 2.0 true))))

(event Custom|Airplane%20Sound
  (bind _returnvalue (Transformation|GetActorLocation))
  ;[1 1 1] Airplane sound effects
  (Networking|SwitchHasAuthority
    (:Remote
      (Audio|PlaySoundatLocation "/Game/Audio/Ambient/Aircrafts/FlybyNew/jet_flyby_distant_long_new_10.jet_flyby_distant_long_new_10" _returnvalue "0, 0, 0" 0.4)
      (Utilities|FlowControl|Delay 2.0)
      (Audio|PlaySoundatLocation "/Game/Audio/Ambient/Aircrafts/FlybyNew/jet_flyby_distant_long_new_01.jet_flyby_distant_long_new_01" _returnvalue "0, 0, 0" 0.4))))

(event Custom|Play%20Beginning%20Sounds.
  (params (Player :type Player%20Controller%20Object%20Reference))
  (bind _returnvalue (Transformation|GetActorLocation Player))
  ;[1 1 1] Radio Chatter
  (Audio|PlaySoundatLocation "/Game/Audio/Deployables/FOB/Radios/US/military_chatter_14_Cue.military_chatter_14_Cue" _returnvalue)
  (Utilities|FlowControl|Delay 1e+01)
  (Audio|PlaySoundatLocation "/Game/Audio/Deployables/FOB/Radios/US/military_chatter_16_Cue.military_chatter_16_Cue" _returnvalue))

(event Custom|Move%20Gun/Spawn%20Plane
  (params (Direction :type Rotator) (Hitloc :type Vector))
  ;[1 1 1] Calculate Positions
  (Networking|SwitchHasAuthority
    (:Authority
      (Transformation|SetActorTransform (Utilities|MakeTransformfromRotandHitPos Hitloc Direction 2e+04 -1e+03) false true))
    (:Remote
      (bind _returnvalue (Game|SpawnActorfromClass "/SquadOps/factionbps/factions/factionfobs/US/A-10/BP_A10Flyover.BP_A10Flyover_C" (Utilities|MakeBomberTransform Hitloc Direction 2e+05 -5e+05) "Undefined" 0 0))
      (Default|StartRun _returnvalue true))))

(event Custom|Begin%20Gunrun
  (params (Direction :type Rotator) (Hitloc :type Vector) (PlayerReference :type Player%20Controller%20Object%20Reference))
  (bind _returnvalue (Transformation|GetActorLocation))
  ;[1 1 1] Trace all impacts before hand
  (CallFunction|MoveGun/SpawnPlane Direction Hitloc)
  (CallFunction|PlayBeginningSounds. PlayerReference)
  (Utilities|FlowControl|Delay 8.0)
  (CallFunction|AirplaneSound)
  (Utilities|FlowControl|Delay 7.0)
  (Utilities|Array|Clear (Variables|Default|GetHit))
  (for _index (range 1 5)
    (bind _outhit (Collision|LineTraceByChannel _returnvalue (+ _returnvalue (* (Utilities|Innacuracy 5.0) 999999999.0)) "TraceTypeQuery1" false 0 "None"))
    (Utilities|Array|Add (Variables|Default|GetHit) (.Location (Collision|BreakHitResult _outhit))))
  ;[1 1 1] Splash effect and sounds on every client, damage effect on server
  (CallFunction|Explode)
  (bind _index_2 (Utilities|ForLoopwithDelay 2 4 0.2)
    (:Loop%20Body
      (Class|SQBlueprintLibrary|ApplyRadialDamagewithFalloff 5e+02 0.0 (Utilities|Array|Get(acopy) (Variables|Default|GetHit) _index_2) 1.2e+03 5e+02 3e+03 1.0 "/Game/Gameplay/DamageTypes/BP_RPG_HEAT.BP_RPG_HEAT_C" 0 0 0 true "ECC_GameTraceChannel8"))
    (:Completed
      ;[1 1 1] Plays sound for all clients, waits, then  destroys the gun
      (Utilities|FlowControl|Delay 2.0)
      (Networking|SwitchHasAuthority
        (:Authority
          (Actor|DestroyActor))))))

(fn ConstructionScript)