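; BP_A10Flyover is an A-10 flyover actor for the US faction's fire support, pushed along its forward vector by a fast looping timer.
; StartRun either just destroys the plane after a delay for bomb runs, or triggers timed gun smoke and a pull-up.
; A local delayed-loop macro paces the smoke emitters and stepped rotations, with the later rotations and final destroy nested inside loop bodies.
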(event Custom|Move
  ;[1 1 1] Event triggered by timer, moves the plane 20 units on it's forward axis
  (Transformation|SetActorLocation (+ (Transformation|GetActorLocation) (* (Transformation|GetActorForwardVector) 2e+01)) false true))

(event Custom|Gunsmoke
  ;[1 1 1] Gun Smoke. Triggered by the Call In BP
  (Utilities|ForLoopwithDelay 50 100 0.01
    (:Loop%20body
      (Effects|SpawnEmitteratLocation "/SquadOps/factionbps/factions/factionfobs/US/A-10/A10Smoke.A10Smoke" (Transformation|GetActorLocation) "5.000000, 0, 0"))))

(event Custom|Pull%20Up
  ;[1 1 1] Pulls up out of the dive.
  (Utilities|ForLoopwithDelay 1 45 0.05
    (:Loop%20body
      (Transformation|AddActorLocalRotation "1.000000, 0,-1.000000" false false))
    (:Completed
      (Utilities|FlowControl|Delay 12.0)
      ;[1 1 1] Rotates back to flying flat
      (Utilities|ForLoopwithDelay 1 45 0.05
        (:Loop%20body
          (Transformation|AddActorLocalRotation "0.000000, 0,-2.000000" false false)
          (Utilities|FlowControl|Delay 5.0)
          ;[1 1 1] Do a barrel roll
          (Utilities|ForLoopwithDelay 1 45 0.05
            (:Loop%20body
              (Transformation|AddActorLocalRotation "0.000000, 0,1.000000" false false)
              ;[1 1 1] Delete Actor
              (Utilities|FlowControl|Delay 1e+01)
              (Actor|DestroyActor))))))))

(event Custom|Start%20Run
  (params (Bomb? :type Boolean))
  (if Bomb?
    (Utilities|FlowControl|Delay 5e+01)
    (Actor|DestroyActor)
    (else
      (Utilities|FlowControl|Delay 14.0)
      (CallFunction|Gunsmoke)
      (Utilities|FlowControl|Delay 4.0)
      (CallFunction|PullUp))))

(event EventBeginPlay
  ;[1 1 1] Starts a timer to move the plane every .001 seconds
  (Utilities|Time|SetTimerbyEvent (delegate Custom|Move) 0.001 true))

(fn ConstructionScript)