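; Game mode Blueprint that handles player requests to place deployables and destroys all forward bases when play ends.
; A request is validated by a camera-channel line trace to the player's pawn and a maximum distance check.
; It then spawns the deployable for the player's team, tests placement and, where required, asks the nearest FOB to accept it.
; Accepted deployables are marked placed; spawned ones that fail are destroyed.
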(event Custom|RequestPlaceDeployable
  (params (DeployableClass :type SQ%20Deployable%20Class%20Reference) (SpawnLocation :type Transform) (PlayerController :type SQ%20Player%20Controller%20Object%20Reference))
  (bind _teamstate (Variables|/Script/Squad.SQPlayerController|GetTeamState PlayerController))
  (bind _id (Variables|/Script/Squad.SQTeamState|GetId _teamstate))
  (bind _returnvalue (Utilities|ValidateRequestPlaceDeployable SpawnLocation PlayerController))
  (if _returnvalue
    (bind _returnvalue_2 (Game|SpawnActorfromClass DeployableClass SpawnLocation "AlwaysSpawn" 0 _id false (Pawn|GetControlledPawn PlayerController)))
    (Class|SQDeployable|SetTeam _returnvalue_2 _id)
    (bind _returnvalue_3 (Class|SQDeployable|IsValidPlacement _returnvalue_2))
    (if _returnvalue_3
      (if (Variables|/Script/Squad.SQDeployable|GetbRequiresFOB _returnvalue_2)
        (Utilities|IsValid (Class|SQDeployable|GetNearestFOB _returnvalue_2 true)
          (:Is%20Valid
            (bind _returnvalue_4 (Class|SQForwardBase|TryAcceptPlacement (Class|SQDeployable|GetNearestFOB _returnvalue_2 true) _returnvalue_2))
            (if _returnvalue_4
              (Class|SQDeployable|Placed _returnvalue_2 :!label _label)
              (else
                (Actor|DestroyActor _returnvalue_2 :!label _label_2))))
          (:Is%20Not%20Valid
            (goto _label_2)))
        (else
          (goto _label)))
      (else
        (Actor|DestroyActor _returnvalue_2)))))

(event EventBeginPlay)

(event EventEndPlay
  (params (EndPlayReason :type EEndPlayReason%20Enum :default "Destroyed"))
  (|CallParentFunction EndPlayReason)
  (bind _outactors (Actor|GetAllActorsOfClass "/Script/Squad.SQForwardBase"))
  (for _array_element _outactors
    (Actor|DestroyActor _array_element)))

(fn ConstructionScript)

(fn GetIDforTeam
  (params (Team :type SQ%20Team%20Object%20Reference))
  (return (Utilities|Array|FindItem (Variables|Default|GetIndexedTeams) Team)))